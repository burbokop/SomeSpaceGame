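; Player character with six-degree-of-freedom flight controls on a physics mesh and interaction with objects ahead of the camera.
; Movement inputs add linear velocity along the mesh's own axes.
; Roll, yaw and pitch either apply torque or directly rotate the mesh, depending on an InertialRotation flag flipped by the CameraMode action.
; A looping timer has the Interactor select what is in front of the camera, and Interact triggers it.
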(event `InputAxis|Move Up / Down`
  (params (AxisValue :type "Float (single-precision)"))
  (bind __mesh (`self. Mesh`))
  (`PrimitiveComponent.SetPhysicsLinearVelocity` __mesh (* (`SceneComponent.GetUpVector` __mesh) (* AxisValue 10.0)) true "None"))

(event `InputAxis|Move Right / Left`
  (params (AxisValue :type "Float (single-precision)"))
  (bind __mesh (`self. Mesh`))
  (`PrimitiveComponent.SetPhysicsLinearVelocity` __mesh (* (`SceneComponent.GetRightVector` __mesh) (* AxisValue 10.0)) true "None"))

(event `InputAxis|Move Forward / Backward`
  (params (AxisValue :type "Float (single-precision)"))
  (bind __mesh (`self. Mesh`))
  (`PrimitiveComponent.SetPhysicsLinearVelocity` __mesh (* (`SceneComponent.GetForwardVector` __mesh) (* AxisValue 10.0)) true "None"))

(event `InputAxis|Roll`
  (params (AxisValue :type "Float (single-precision)"))
  (bind __mesh (`self. Mesh`))
  (bind __mesh_2 (`self. Mesh`))
  ;[1 1 1] roll
  (if (`self.inertialRotation`)
    (`PrimitiveComponent.AddTorqueInDegrees` __mesh (* (* (`SceneComponent.GetForwardVector` __mesh) -1.0) (* 500.0 AxisValue)) "None" true)
    (else
      (`SceneComponent.K2_SetWorldRotation` __mesh_2 (`KismetMathLibrary.ComposeRotators` (`KismetMathLibrary.MakeRotator` (* AxisValue 1.0)) (`SceneComponent.RelativeRotation` __mesh_2)) false false))))

(event `InputAxis|Turn Right / Left Mouse`
  (params (AxisValue :type "Float (single-precision)"))
  (bind __mesh (`self. Mesh`))
  (bind __mesh_2 (`self. Mesh`))
  ;[1 1 1] rotate left / right
  (if (`self.inertialRotation`)
    (`PrimitiveComponent.AddTorqueInDegrees` __mesh (* (`SceneComponent.GetUpVector` __mesh) (* 500.0 AxisValue)) "None" true)
    (else
      (`SceneComponent.K2_SetWorldRotation` __mesh_2 (`KismetMathLibrary.ComposeRotators` (`KismetMathLibrary.MakeRotator` 0.0 0.0 (* AxisValue 1.0)) (`SceneComponent.RelativeRotation` __mesh_2)) false false))))

(event `InputAxis|Look Up / Down Mouse`
  (params (AxisValue :type "Float (single-precision)"))
  (bind __mesh (`self. Mesh`))
  (bind __mesh_2 (`self. Mesh`))
  ;[1 1 1] rotate up / down
  (if (`self.inertialRotation`)
    (`PrimitiveComponent.AddTorqueInDegrees` __mesh (* (`SceneComponent.GetRightVector` __mesh) (* 500.0 AxisValue)) "None" true)
    (else
      (`SceneComponent.K2_SetWorldRotation` __mesh_2 (`KismetMathLibrary.ComposeRotators` (`KismetMathLibrary.MakeRotator` 0.0 (* AxisValue -1.0)) (`SceneComponent.RelativeRotation` __mesh_2)) false false))))

(event `InputAction|CameraMode`
  (params (Key :type "Key Structure"))
  (:`Released`
    (bind _isa (`/Engine/EditorBlueprintResources/StandardMacros.FlipFlop`)
      (:`A`
        _)
      (:`B`
        _))
    (set `self.inertialRotation` _isa)))

(event `self.ReceiveBeginPlay`
  (`KismetSystemLibrary.K2_SetTimerDelegate` (delegate `CheckTrace`) 0.1 true))

(event `CheckTrace`
  (`/Game/Interaction/PB_Interactor.Select In Front Of Camera` (`self.Interactor`) (`self.Camera`) 400.0))

(event `InputAction|Interact`
  (params (Key :type "Key Structure"))
  (:`Released`
    (`/Game/Interaction/PB_Interactor.Interact With Selected` (`self.Interactor`))))

(fn `UserConstructionScript`)